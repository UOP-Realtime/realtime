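; VR biome selector actor that spawns two biome previews and loads the level of the one placed in its zone.
; On overlap it releases the grabbed preview, snaps and attaches it, and stores its level and offsets.
; Timelines then sink the selector and fade scene lights alongside the pawn's scene teleport.
; Afterward it streams in a level instance, destroys previews and hides itself and the first StaticMeshActor found.
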(event OnComponentBeginOverlap(SelectorPlacementZone)
  (params (OverlappedComponent :type Primitive%20Component%20Object%20Reference) (OtherActor :type Actor%20Object%20Reference) (OtherComp :type Primitive%20Component%20Object%20Reference) (OtherBodyIndex :type Integer) (bFromSweep :type Boolean) (SweepResult :type Hit%20Result%20Structure%20%28by%20ref%29))
  (bind _asbiome_preview_base (Utilities|Casting|CastToBiomePreviewBase OtherActor))
  (bind _breleased (Default|TryRelease (Variables|/Game/Blueprints/BiomePreviews/BiomePreviewBase.BiomePreviewBase_C|GetGrabComponent _asbiome_preview_base)))
  (if _breleased
    (bind _asvrpawn (Utilities|Casting|CastToVRPawn (Game|Player|GetPlayerPawn 0)))
    (Variables|/Game/VRTemplate/Blueprints/VRPawn.VRPawn_C|SetHeldComponentLeft _asvrpawn 0)
    (Variables|/Game/VRTemplate/Blueprints/VRPawn.VRPawn_C|SetHeldComponentRight _asvrpawn 0)
    (Physics|SetSimulatePhysics (Variables|/Game/Blueprints/BiomePreviews/BiomePreviewBase.BiomePreviewBase_C|GetPreviewBiomeDome_SM _asbiome_preview_base) false)
    (Transformation|SetActorTransform _asbiome_preview_base (Transformation|GetWorldTransform (Variables|Default|GetSelected%20Biome%20Placement%20Point)) false true)
    (Transformation|AttachActorToActor _asbiome_preview_base self "None" "KeepWorld" "KeepWorld" "KeepWorld" false)
    (Variables|Default|SetLevel%20To%20Load (Variables|/Game/Blueprints/BiomePreviews/BiomePreviewBase.BiomePreviewBase_C|GetOwned%20Level _asbiome_preview_base))
    (Variables|Default|SetLevel%20Location%20Offset (Variables|/Game/Blueprints/BiomePreviews/BiomePreviewBase.BiomePreviewBase_C|GetLocation%20Offset _asbiome_preview_base))
    (Variables|Default|SetLevel%20Rotation%20Offset (Variables|/Game/Blueprints/BiomePreviews/BiomePreviewBase.BiomePreviewBase_C|GetRotation%20Offset _asbiome_preview_base))
    (CallFunction|Hide)))

(event Custom|Hide
  (bind _returnvalue (Transformation|GetActorLocation))
  (bind _asvrpawn (Utilities|Casting|CastToVRPawn (Game|Player|GetPlayerPawn 0))
    (:then
      (Default|StartSceneTeleport _asvrpawn))
    (:CastFailed
      _))
  (CallFunction|RemoveLevelStuff)
  (bind _alpha (Timeline|Hide%20Basin PlayFromStart)
    (:Update
      (Transformation|SetActorLocation (Math|Vector|MakeVector (.x _returnvalue) (.y _returnvalue) (Math|Float|Lerp 0.0 -1.5e+02 _alpha)) false false))
    (:Finished
      (Class|LevelStreamingDynamic|LoadLevelInstance (Utilities|String|ToString(Name) (Variables|Default|GetLevel%20To%20Load)) (Variables|Default|GetLevel%20Location%20Offset) (Variables|Default|GetLevel%20Rotation%20Offset) "" "/Script/Engine.LevelStreamingDynamic" false)
      (bind _returnvalue_2 (Actor|GetActorOfClass "/Script/Engine.StaticMeshActor"))
      (Rendering|SetActorHiddenInGame _returnvalue_2 true)
      (bind _outactors (Actor|GetAllActorsOfClass "/Game/Blueprints/BiomePreviews/BiomePreviewBase.BiomePreviewBase_C"))
      (for _array_element _outactors
        (Actor|DestroyActor _array_element))
      (Rendering|SetActorHiddenInGame true))))

(event Custom|Remove%20Level%20Stuff
  (bind _returnvalue (Actor|GetActorOfClass "/Script/Engine.DirectionalLight"))
  (bind _returnvalue_2 (Actor|GetActorOfClass "/Script/Engine.SkyLight"))
  (bind _alpha (Timeline|FadeOutLevelStuff PlayFromStart)
    (:Update
      (Rendering|Components|Light|SetIntensity (Variables|/Script/Engine.Light|GetLightComponent _returnvalue) (Math|Float|Lerp 2.0 0.0 _alpha))
      (Rendering|Components|Light|SetIntensity (Variables|/Script/Engine.SkyLight|GetLightComponent _returnvalue_2) (Math|Float|Lerp 0.2 0.0 _alpha)))
    (:Finished
      (Rendering|SetActorHiddenInGame _returnvalue true))))

(event EventBeginPlay
  (Game|SpawnActorfromClass (Variables|Default|GetBiome%201) (Math|Transform|MakeTransform (Transformation|GetWorldLocation (Variables|Default|GetBiome%201%20Spawn)) "0, 0, 0" "1.000000,1.000000,1.000000") "AlwaysSpawn" "MultiplyWithRoot" 0 0)
  (Game|SpawnActorfromClass (Variables|Default|GetBiome%202) (Math|Transform|MakeTransform (Transformation|GetWorldLocation (Variables|Default|GetBiome%202%20Spawn)) "0, 0, 0" "1.000000,1.000000,1.000000") "AlwaysSpawn" "MultiplyWithRoot" 0 0))

(event Collision|EventActorBeginOverlap
  (params (OtherActor :type Actor%20Object%20Reference)))

(event EventTick
  (params (DeltaSeconds :type Float%20%28single-precision%29)))

(fn ConstructionScript)