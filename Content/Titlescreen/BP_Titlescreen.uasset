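; Titlescreen actor that plays an intro animation with a growing sphere and a logo opacity fade.
; BeginPlay sets a delayed timer event, though its bound function is not shown.
; ScaleSphere uses a timeline to enlarge the Sphere, then calls FadeLogo on completion.
; FadeLogo creates a dynamic material instance on the Logo and drives its Opacity parameter from a second timeline.
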(event Custom|FadeLogo
  (bind _returnvalue (Rendering|Material|CreateDynamicMaterialInstance (Variables|Default|GetLogo) 0 "/Game/Materials/M_TitlescreenLogo.M_TitlescreenLogo" "None" :!class /Script/Engine.PrimitiveComponent))
  (bind _newtrack_0 (Timeline|OpacityFade Play)
    (:Update
      (Rendering|Material|SetScalarParameterValue _returnvalue "Opacity" _newtrack_0 :!class /Script/Engine.MaterialInstanceDynamic))))

(event Custom|ScaleSphere
  (bind _newtrack_0 (Timeline|Scale Play)
    (:Update
      (Transformation|SetWorldScale3D (Variables|Default|GetSphere) (Math|Vector|Lerp(Vector) "25.000000,25.000000,25.000000" "250.000000,250.000000,250.000000" _newtrack_0)))
    (:Finished
      (CallFunction|FadeLogo))))

(event EventBeginPlay
  (Utilities|Time|SetTimerbyEvent (EventDispatchers|CreateEvent :!event Custom|ScaleSphere) 5.0))

(event Collision|EventActorBeginOverlap
  (params (OtherActor :type Actor%20Object%20Reference)))

(event EventTick
  (params (DeltaSeconds :type Float%20%28single-precision%29)))

(fn ConstructionScript)